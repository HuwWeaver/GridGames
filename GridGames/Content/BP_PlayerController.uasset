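; Player controller for a chess-style board game that lets the player select and move pieces with the mouse cursor.
; Left click alternates between two cursor traces on separate object types: the first picks a game piece, the next looks for a grid tile.
; A free tile passes the move to BP_ChessGM's MovePiece and clears the selection; an occupied or missed tile only prints debug text, keeping the piece selected.
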(event EventBeginPlay
  (Variables|Default|SetbShowMouseCursor true))

(event Input|MouseEvents|LeftMouseButton
  (params (Key :type Key%20Structure :default "None"))
  (bind _array (Utilities|Array|MakeArray "ObjectTypeQuery8"))
  (bind _array_2 (Utilities|Array|MakeArray "ObjectTypeQuery7"))
  (bind (_hitresult _returnvalue) (Class|PlayerController|GetHitResultUnderCursorforObjects _array true))
  (bind (_hitresult_2 _returnvalue_2) (Class|PlayerController|GetHitResultUnderCursorforObjects _array_2 true))
  (bind _hitactor (Collision|BreakHitResult _hitresult))
  (bind _asbp_grid_tile (Utilities|Casting|CastToBP_GridTile _hitactor))
  (:Pressed
    (if (Variables|Default|GetGamePieceSelected)
      (if _returnvalue
        (Development|PrintString "Tile Hit" true true "(R=0.049640,G=1.000000,B=0.000000,A=1.000000)")
        (if (Variables|/Game/BP_GridTile.BP_GridTile_C|GetOccupied _asbp_grid_tile)
          (Development|PrintString "Tile Is Occupied" true true "(R=1.000000,G=0.064799,B=0.000000,A=1.000000)")
          (else
            (Development|PrintString "Tile Is Free" true true "(R=0.049640,G=1.000000,B=0.000000,A=1.000000)")
            (bind _asbp_chess_gm (Utilities|Casting|CastToBP_ChessGM (Game|GetGameMode)))
            (Default|MovePiece _asbp_chess_gm (Variables|Default|GetSelected%20Game%20Piece) _asbp_grid_tile)
            (Variables|Default|SetGamePieceSelected false)
            (Variables|Default|SetSelected%20Game%20Piece 0)))
        (else
          (Development|PrintString "Tile Not Found" true true "(R=1.000000,G=0.064799,B=0.000000,A=1.000000)")))
      (elif _returnvalue_2
        (Development|PrintString "Game Piece Hit" true true "(R=0.049640,G=1.000000,B=0.000000,A=1.000000)")
        (Variables|Default|SetGamePieceSelected true)
        (bind _asbp_game_piece (Utilities|Casting|CastToBP_GamePiece (.HitActor (Collision|BreakHitResult _hitresult_2))))
        (Variables|Default|SetSelected%20Game%20Piece _asbp_game_piece)
        (else
          (Development|PrintString "Game Piece Not Found" true true "(R=1.000000,G=0.064799,B=0.000000,A=1.000000)"))))))

(fn ConstructionScript)