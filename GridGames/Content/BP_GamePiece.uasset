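; BP_GamePiece is a board game piece actor with a mesh and a text label, set up at runtime through an Init event.
; Init takes a properties struct, writes the piece name to the TextRender and stores the starting coordinate as CurrentCoordinate.
; The White flag picks a solid white or black material and gives the label the opposite color for contrast.
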(event Custom|Init
  (params (Properties :type F%20Piece%20Properties%20Structure))
  (bind (_name _white_ _startingcoordinate) (Utilities|Struct|BreakF_PieceProperties Properties))
  (bind _textrender (Variables|Default|GetTextRender))
  (bind _staticmesh (Variables|Default|GetStaticMesh))
  (Rendering|Components|TextRender|SetText (Variables|Default|GetTextRender) _name)
  (Variables|Default|SetCurrentCoordinate _startingcoordinate)
  (if _white_
    (Rendering|Material|SetMaterial _staticmesh 0 "/Game/LevelPrototyping/Materials/MI_Solid_White.MI_Solid_White")
    (Rendering|Components|TextRender|SetTextRenderColor _textrender (Math|Color|MakeColor 0 0 0 255))
    (else
      (Rendering|Material|SetMaterial _staticmesh 0 "/Game/LevelPrototyping/Materials/MI_Solid_Black.MI_Solid_Black")
      (Rendering|Components|TextRender|SetTextRenderColor _textrender (Math|Color|MakeColor 255 255 255 255)))))

(fn ConstructionScript)