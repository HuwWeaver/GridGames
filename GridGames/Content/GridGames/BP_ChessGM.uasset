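; Chess game manager that sets up the starting pieces on a tile grid and repositions them when moved.
; On BeginPlay it finds the BP_GridManager, then spawns and initializes a BP_GamePiece for each ChessSetup data table row.
; Starting coordinates are X/Y-swapped, scaled by tile size and rotated with the grid, then given an unrotated half-tile and height offset.
; MovePiece snaps a piece to a target tile with that offset, without rule checks.
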(event Custom|GameSetup
  (bind _gridmanagerref (Variables|Default|GetGridManagerRef))
  (bind _returnvalue (Transformation|GetActorTransform _gridmanagerref))
  (bind _tilesize (Variables|/Game/GridGames/BP_GridManager.BP_GridManager_C|GetTileSize _gridmanagerref))
  (bind _returnvalue_2 (/ _tilesize 2.0))
  (bind _outrownames (DataTable|GetDataTableRowNames "/Game/GridGames/ChessSetup.ChessSetup"))
  (for _array_element _outrownames
    (bind _returnvalue_3 (Utilities|GetDataTableRow "/Game/GridGames/ChessSetup.ChessSetup" _array_element)
      (:then
        (bind _returnvalue_4 (Game|SpawnActorfromClass "/Game/GridGames/BP_GamePiece.BP_GamePiece_C" (Math|Transform|MakeTransform (+ (+ (.location _returnvalue) (Math|Vector|RotateVector (Math|Vector|MakeVector (* (.y (.StartingCoordinate (Utilities|Struct|BreakF_PieceProperties _returnvalue_3))) _tilesize) (* (.x (.StartingCoordinate (Utilities|Struct|BreakF_PieceProperties _returnvalue_3))) _tilesize) 0.0) (.rotation _returnvalue))) (Math|Vector|MakeVector _returnvalue_2 _returnvalue_2 1e+02)) (.rotation _returnvalue) "1.000000,1.000000,1.000000") "Undefined" "OverrideRootScale" 0 0))
        (Default|Init _returnvalue_4 _returnvalue_3)))))

(event Custom|MovePiece
  (params (Piece :type BP%20Game%20Piece%20Object%20Reference) (NewTile :type BP%20Grid%20Tile%20Object%20Reference))
  (bind _gridmanagerref (Variables|Default|GetGridManagerRef))
  (bind _tilesize (Variables|/Game/GridGames/BP_GridManager.BP_GridManager_C|GetTileSize _gridmanagerref))
  (bind _returnvalue (/ _tilesize 2.0))
  (Development|PrintString "Move Piece")
  (Transformation|SetActorLocation Piece (+ (Transformation|GetActorLocation NewTile) (Math|Vector|MakeVector _returnvalue _returnvalue 1e+02)) false false))

(event EventBeginPlay
  (bind _returnvalue (Actor|GetActorOfClass "/Game/GridGames/BP_GridManager.BP_GridManager_C"))
  (Variables|Default|SetGridManagerRef _returnvalue)
  (CallFunction|GameSetup))

(fn ConstructionScript)