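; BP_GridGameGM is a base game mode for grid board games that handles piece selection, move validation and capturing.
; PieceSelected walks the piece's move list, highlighting valid tiles from the 3D-coordinate GridMap as single steps or boundless rays that stop at blockers.
; Occupied tiles highlight only for opposing pieces when the move can capture.
; TryMovePiece accepts tiles flagged ValidMove, destroys any occupant, moves the piece, then calls OnPieceMoved.
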(event Custom|TryMovePiece
  (params (Selected%20Piece :type BP%20Game%20Piece%20Object%20Reference) (Target%20Tile :type BP%20Grid%20Tile%20Object%20Reference))
  ;[0.01556 0.15 0.001029 0.5] Game Mode Base Class
  ;;[0.03125 0.03125 0.03125 0.5] Try Move Piece:
  ;; 1. Check if tile within allowed movement parameters
  ;; 2. Check if tile is free
  ;; 3. If not free, check if can capture piece
  (if (Variables|/Script/GridGames.GridTile|GetbValidMove Target%20Tile)
    (Development|PrintString "Move is Valid" true true "(R=0.049640,G=1.000000,B=0.000000,A=1.000000)")
    (if (Variables|/Script/GridGames.GridTile|GetbOccupied Target%20Tile)
      (Development|PrintString "Capturing Move" true true "(R=0.049640,G=1.000000,B=0.000000,A=1.000000)")
      (Actor|DestroyActor (Variables|/Game/GridGames/BP_GridTile.BP_GridTile_C|GetOccupyingPiece Target%20Tile)))
    (Class|GamePiece|Move Selected%20Piece Target%20Tile (Variables|Default|GetTileSize))
    (Default|CallOnPieceMoved)
    (else
      (Development|PrintString "Invalid Move" true true "(R=1.000000,G=0.064799,B=0.000000,A=1.000000)"))))

(event Custom|PieceSelected
  (params (Selected%20Piece :type BP%20Game%20Piece%20Object%20Reference))
  (bind _currentcoordinate (Variables|/Script/GridGames.GamePiece|GetCurrentCoordinate Selected%20Piece))
  (bind _setupproperties (Variables|/Script/GridGames.GamePiece|GetSetupProperties Selected%20Piece))
  (bind _bwhite (Utilities|Struct|BreakPieceSetupProperties _setupproperties))
  (for _array_element (Utilities|Struct|BreakPieceMovementData (Variables|/Script/GridGames.GamePiece|GetMovementData Selected%20Piece))
    ;[0.7708 0.3753 0 0.5] Loop Body different in each gamemode
    (switch Utilities|FlowControl|Switch|SwitchonEMovementTypes (.MoveType (Utilities|Struct|BreakPieceMovementProperties _array_element))
      (:Step
        (CallFunction|ShowStepMove _bwhite _currentcoordinate (.MovementVector (Utilities|Struct|BreakPieceMovementProperties _array_element)) (.bCanCapture (Utilities|Struct|BreakPieceMovementProperties _array_element))))
      (:BoundlessRange
        (CallFunction|ShowBoundlessMoves _bwhite _currentcoordinate (.MovementVector (Utilities|Struct|BreakPieceMovementProperties _array_element)) (.bCanCapture (Utilities|Struct|BreakPieceMovementProperties _array_element)))))))

(fn ConstructionScript)

(fn ShowBoundlessMoves
  (params (White? :type Boolean) (StartingCoordinate :type Vector) (MovementVector :type Vector) (Move%20Can%20Capture? :type Boolean))
  (LocalVariables|SetNewX (+ (.x StartingCoordinate) (.x MovementVector)))
  (LocalVariables|SetNewY (+ (.y StartingCoordinate) (.y MovementVector)))
  (LocalVariables|SetNewZ (+ (.z StartingCoordinate) (.z MovementVector)))
  (while (.ReturnValue (Utilities|Map|Find (Variables|Default|GetGridMap) (Math|Vector|MakeVector (Math|Conversions|ToFloat(Integer) (LocalVariables|GetNewX)) (Math|Conversions|ToFloat(Integer) (LocalVariables|GetNewY)) (Math|Conversions|ToFloat(Integer) (LocalVariables|GetNewZ)))))
    (if (Variables|/Script/GridGames.GridTile|GetbOccupied (.Value (Utilities|Map|Find (Variables|Default|GetGridMap) (Math|Vector|MakeVector (Math|Conversions|ToFloat(Integer) (LocalVariables|GetNewX)) (Math|Conversions|ToFloat(Integer) (LocalVariables|GetNewY)) (Math|Conversions|ToFloat(Integer) (LocalVariables|GetNewZ))))))
      (if (== White? (Utilities|Struct|BreakPieceSetupProperties (Variables|/Script/GridGames.GamePiece|GetSetupProperties (Variables|/Game/GridGames/BP_GridTile.BP_GridTile_C|GetOccupyingPiece (.AsBP%20Grid%20Tile (Utilities|Casting|CastToBP_GridTile (.Value (Utilities|Map|Find (Variables|Default|GetGridMap) (Math|Vector|MakeVector (Math|Conversions|ToFloat(Integer) (LocalVariables|GetNewX)) (Math|Conversions|ToFloat(Integer) (LocalVariables|GetNewY)) (Math|Conversions|ToFloat(Integer) (LocalVariables|GetNewZ)))))))))))
        _
        (elif Move%20Can%20Capture?
          (Default|ShowValidMove (.AsBP%20Grid%20Tile (Utilities|Casting|CastToBP_GridTile (.Value (Utilities|Map|Find (Variables|Default|GetGridMap) (Math|Vector|MakeVector (Math|Conversions|ToFloat(Integer) (LocalVariables|GetNewX)) (Math|Conversions|ToFloat(Integer) (LocalVariables|GetNewY)) (Math|Conversions|ToFloat(Integer) (LocalVariables|GetNewZ))))))))))
      (return)
      (else
        (Default|ShowValidMove (.AsBP%20Grid%20Tile (Utilities|Casting|CastToBP_GridTile (.Value (Utilities|Map|Find (Variables|Default|GetGridMap) (Math|Vector|MakeVector (Math|Conversions|ToFloat(Integer) (LocalVariables|GetNewX)) (Math|Conversions|ToFloat(Integer) (LocalVariables|GetNewY)) (Math|Conversions|ToFloat(Integer) (LocalVariables|GetNewZ))))))))
        (LocalVariables|SetNewX (+ (LocalVariables|GetNewX) (.x MovementVector)))
        (LocalVariables|SetNewY (+ (LocalVariables|GetNewY) (.y MovementVector)))
        (LocalVariables|SetNewZ (+ (LocalVariables|GetNewZ) (.z MovementVector))))))
  (return))

(fn ShowStepMove
  (params (White? :type Boolean) (Starting%20Coordinate :type Vector%20%28by%20ref%29) (Movement%20Vector :type Vector%20%28by%20ref%29) (Move%20Can%20Capture? :type Boolean))
  (bind _returnvalue (+ Starting%20Coordinate Movement%20Vector))
  (bind _gridmap (Variables|Default|GetGridMap))
  (bind (_value _returnvalue_2) (Utilities|Map|Find _gridmap _returnvalue))
  (bind _asbp_grid_tile (Utilities|Casting|CastToBP_GridTile _value))
  (if _returnvalue_2
    (if (Variables|/Script/GridGames.GridTile|GetbOccupied _value)
      (if (== White? (Utilities|Struct|BreakPieceSetupProperties (Variables|/Script/GridGames.GamePiece|GetSetupProperties (Variables|/Game/GridGames/BP_GridTile.BP_GridTile_C|GetOccupyingPiece _asbp_grid_tile))))
        _
        (elif Move%20Can%20Capture?
          (Default|ShowValidMove _asbp_grid_tile :!label _label)))
      (else
        (goto _label))))
  (return))