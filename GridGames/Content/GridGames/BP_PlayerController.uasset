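; Player controller for a grid-based board game that lets the player select and move game pieces with the mouse.
; Left click traces under the cursor: with nothing selected it picks a game piece and notifies GridGameGameMode, otherwise it asks the game mode to move that piece to the clicked tile.
; Right click fires the deselect call and clears the selection.
; Debug strings print each hit or miss.
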(event Input|MouseEvents|LeftMouseButton
  (params (Key :type Key%20Structure :default "None"))
  (bind _array (Utilities|Array|MakeArray "ObjectTypeQuery8"))
  (bind _array_2 (Utilities|Array|MakeArray "ObjectTypeQuery7"))
  (bind (_hitresult _returnvalue) (Class|PlayerController|GetHitResultUnderCursorforObjects _array true))
  (bind (_hitresult_2 _returnvalue_2) (Class|PlayerController|GetHitResultUnderCursorforObjects _array_2 true))
  (:Pressed
    (if (Variables|Default|GetGamePieceSelectedBP)
      (if _returnvalue
        (Development|PrintString "Tile Hit" true true "(R=0.049640,G=1.000000,B=0.000000,A=1.000000)")
        (bind _asgrid_game_game_mode (Utilities|Casting|CastToGridGameGameMode (Game|GetGameMode)))
        (Class|GridGameGameMode|TryMovePiece _asgrid_game_game_mode (Variables|Default|GetSelected%20Game%20PieceBP) (.AsGrid%20Tile (Utilities|Casting|CastToGridTile (.HitActor (Collision|BreakHitResult _hitresult)))))
        (else
          (Development|PrintString "Tile Not Found" true true "(R=1.000000,G=0.064799,B=0.000000,A=1.000000)")))
      (elif _returnvalue_2
        (Development|PrintString "Game Piece Hit" true true "(R=0.049640,G=1.000000,B=0.000000,A=1.000000)")
        (bind _asgame_piece (Utilities|Casting|CastToGamePiece (.HitActor (Collision|BreakHitResult _hitresult_2))))
        (Variables|Default|SetSelected%20Game%20PieceBP _asgame_piece)
        (Variables|Default|SetGamePieceSelectedBP true)
        (bind _asgrid_game_game_mode_2 (Utilities|Casting|CastToGridGameGameMode (Game|GetGameMode)))
        (Class|GridGameGameMode|OnPieceSelected _asgrid_game_game_mode_2 (Variables|Default|GetSelected%20Game%20PieceBP))
        (else
          (Development|PrintString "Game Piece Not Found" true true "(R=1.000000,G=0.064799,B=0.000000,A=1.000000)"))))))

(event Input|MouseEvents|RightMouseButton
  (params (Key :type Key%20Structure :default "None"))
  (:Pressed
    (Default|CallOnPieceDeselected)
    (Variables|Default|SetGamePieceSelectedBP false)
    (Variables|Default|SetSelected%20Game%20PieceBP 0)))

(fn ConstructionScript)