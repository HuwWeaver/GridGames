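; Player pawn for a grid-based chess game that shows the piece promotion choice UI to its player.
; ProvidePromotionChoice creates the UMG_Promotion widget for the owning player controller on first use and reuses it afterwards.
; It adds the widget to the viewport and initializes it with the chess piece to promote and that piece's promotion options.
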(event EventProvidePromotionChoice
  (params (Piece :type Game%20Piece%20Object%20Reference))
  (bind _aschess_piece (Utilities|Casting|CastToChessPiece Piece))
  (Utilities|IsValid (Variables|Default|GetPromotionUI)
    (:Is%20Valid
      _)
    (:Is%20Not%20Valid
      (bind _returnvalue (UserInterface|CreateWidget "/Game/GridGames/UI/UMG_Promotion.UMG_Promotion_C" (.AsPlayer%20Controller (Utilities|Casting|CastToPlayerController (Pawn|GetController)))))
      (Variables|Default|SetPromotionUI _returnvalue)))
  (UserInterface|Viewport|AddtoViewport (Variables|Default|GetPromotionUI) 0)
  (Default|Init (Variables|Default|GetPromotionUI) _aschess_piece (Variables|/Script/GridGames.GamePiece|GetPromotionOptions _aschess_piece)))

(fn ConstructionScript)