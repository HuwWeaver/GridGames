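; BP_GridManager is an actor that builds and clears a rectangular grid of BP_GridTile actors for a grid-based game.
; CreateGrid first runs ClearGrid, then spawns tiles across the configured columns and rows, spaced by tile size and aligned to the manager's location and rotation.
; Each tile receives its column and row as coordinates.
; ClearGrid destroys every BP_GridTile in the world, not just those this manager spawned.
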(event Custom|Clear%20Grid
  (Development|PrintString "Clearing Grid Nodes..")
  (bind _outactors (Actor|GetAllActorsOfClass "/Game/GridGames/BP_GridTile.BP_GridTile_C"))
  (for _array_element _outactors
    (Actor|DestroyActor _array_element))
  (Development|PrintString "Grid Cleared!"))

(event Custom|Create%20Grid
  (bind _returnvalue (Transformation|GetActorTransform))
  (bind _tilesize (Variables|Default|GetTileSize))
  (CallFunction|ClearGrid)
  (Development|PrintString "Creating Grid...")
  (for _index (range 0 (- (Variables|Default|GetNumColumns) 1))
    (for _index_2 (range 0 (- (Variables|Default|GetNumRows) 1))
      (bind _returnvalue_2 (Game|SpawnActorfromClass "/Game/GridGames/BP_GridTile.BP_GridTile_C" (Math|Transform|MakeTransform (+ (.location _returnvalue) (Math|Vector|RotateVector (Math|Vector|MakeVector (* _index_2 _tilesize) (* _index _tilesize) 0.0) (.rotation _returnvalue))) (.rotation _returnvalue) "1.000000,1.000000,1.000000") "Undefined" "OverrideRootScale" 0 0))
      (Default|SetCoords _returnvalue_2 (Utilities|Struct|MakeF_Coordinates _index _index_2))))
  (Development|PrintString "Grid Created!"))

(fn ConstructionScript)