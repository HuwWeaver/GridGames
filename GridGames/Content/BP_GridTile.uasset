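; BP_GridTile is a grid tile actor that displays its own coordinates and colors itself in a checkerboard pattern.
; The SetCoords event stores the coordinates and writes them to a text render component as an "(x,y)" label.
; It then picks one of two prototype grid materials for the static mesh based on whether the coordinate sum is even or odd.
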(event Custom|Set%20Coords
  (params (New%20Coords :type F%20Coordinates%20Structure))
  (Variables|Default|SetCoords New%20Coords)
  (Rendering|Components|TextRender|SetText (Variables|Default|GetTextRender) (Utilities|Text|FormatText "({x},{y})" (.x (Variables|Default|GetCoords)) (.y (Variables|Default|GetCoords))))
  (if (== (Math|Integer|%(Integer) (+ (.x (Variables|Default|GetCoords)) (.y (Variables|Default|GetCoords))) 2) 0)
    (Rendering|Material|SetMaterial (Variables|Default|GetStaticMesh) 0 "/Game/PolygonPrototype/Materials/Mat_PolygonPrototype_Global_Grid_01_Inst.Mat_PolygonPrototype_Global_Grid_01_Inst")
    (else
      (Rendering|Material|SetMaterial (Variables|Default|GetStaticMesh) 0 "/Game/PolygonPrototype/Materials/Alts/Mat_PolygonPrototype_Global_Grid_03_Inst.Mat_PolygonPrototype_Global_Grid_03_Inst"))))

(fn ConstructionScript)